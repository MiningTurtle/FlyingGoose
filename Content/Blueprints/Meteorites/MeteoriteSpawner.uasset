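; Meteorite spawner actor that creates meteorites at random points in a box around its moving location.
; On BeginPlay it copies the forward speed of the first FlyingPawn found.
; Tick runs through a Delay between waves, then spawns one actor and offsets the spawner along local X by that speed times delta seconds, so movement also happens only when the delay completes.
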(event `self.ReceiveBeginPlay`
  (bind _outactors (`GameplayStatics.GetAllActorsOfClass` "/Game/Blueprints/FlyingBP/Blueprints/FlyingPawn.FlyingPawn_C"))
  (set `self.movementSpeed` (`/Game/Blueprints/FlyingBP/Blueprints/FlyingPawn.Current forward speed` (`|GetArrayItem` _outactors))))

(event `self.ReceiveTick`
  (params (DeltaSeconds :type "Float (single-precision)"))
  (bind (_returnvalue_x _returnvalue_y _returnvalue_z) (`KismetMathLibrary.BreakVector` (`self.K2_GetActorLocation`)))
  (bind _halfradius (`self.halfRadius`))
  (bind _halfradius_2 (`self.halfRadius`))
  (bind _halfradius_3 (`self.halfRadius`))
  (`KismetSystemLibrary.Delay` (`self.timerInBetweenWaves`))
  ;[1 1 1] spawn meteorite in random location
  (`|SpawnActorFromClass` "/Game/Blueprints/Meteorites/Meteorite.Meteorite_C" (`KismetMathLibrary.MakeTransform` (`KismetMathLibrary.MakeVector` (`KismetMathLibrary.RandomFloatInRange` (- _returnvalue_x _halfradius_2) (+ _halfradius_2 _returnvalue_x)) (`KismetMathLibrary.RandomFloatInRange` (- _returnvalue_y _halfradius_3) (+ _halfradius_3 _returnvalue_y)) (`KismetMathLibrary.RandomFloatInRange` (- _returnvalue_z _halfradius) (+ _halfradius _returnvalue_z)))) "Undefined" "OverrideRootScale" null null)
  (`self.K2_AddActorLocalOffset` (`KismetMathLibrary.MakeVector` (* DeltaSeconds (`self.movementSpeed`)))))

(fn `UserConstructionScript`)