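; Meteorite projectile actor that tumbles as it moves and removes itself on timeout or impact.
; BeginPlay randomizes the ProjectileMovement InitialSpeed, capped at the component's max speed.
; Tick accumulates elapsed time to destroy the actor after TimeAlive and adds a fixed Angle rotation on all axes each frame, not scaled by delta time.
; Sphere1 overlap destroys the meteorite unless the other actor is also a Meteorite.
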(event `self.ReceiveBeginPlay`
  (bind _projectilemovement (`self.ProjectileMovement`))
  ;[1 1 1] random speed
  (set `ProjectileMovementComponent.InitialSpeed` (`KismetMathLibrary.RandomFloatInRange` 800.0 (`MovementComponent.GetMaxSpeed` _projectilemovement)) _projectilemovement))

(event `self.ReceiveTick`
  (params (DeltaSeconds :type "Float (single-precision)"))
  (bind _angle (`self.angle`))
  (`|ExecutionSequence`
    (:`then_0`
      ;[1 1 1] destroy after x amount of time
      (bind _output_get (set `self.elapsedSec` (+ DeltaSeconds (`self.elapsedSec`))))
      (if (>= _output_get (`self.timeAlive`))
        (`self.K2_DestroyActor`)))
    (:`then_1`
      (`self.K2_AddActorWorldRotation` (`KismetMathLibrary.MakeRotator` _angle _angle _angle)))))

(event `self.Sphere1.OnComponentBeginOverlap`
  (params (OverlappedComponent :type "PrimitiveComponent Object Reference") (OtherActor :type "Actor Object Reference") (OtherComp :type "PrimitiveComponent Object Reference") (OtherBodyIndex :type Integer) (bFromSweep :type Boolean) (SweepResult :type "HitResult Structure (by ref)"))
  ;[1 1 1] collision
  (cast `/Game/Blueprints/Meteorites/Meteorite` OtherActor
    (:`CastFailed`
      (`self.K2_DestroyActor`))))

(fn `UserConstructionScript`)