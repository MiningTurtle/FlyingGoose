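; Gun is a turret actor that fires automatically and aims in yaw from an axis input.
; Tick runs through a Delay, spawning a BaseProjectile at BulletLoc about once per second.
; The Rotate event maps AxisInput around a RotAngle offset to TurretMesh world yaw, then clamps it to a half-circle with a swept transform update.
; An interpolation node for smoothing the rotation is left unused.
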(event `self.ReceiveTick`
  (params (DeltaSeconds :type "Float (single-precision)"))
  (set `self.deltaTime` DeltaSeconds)
  (`KismetSystemLibrary.Delay` 1.0)
  (`|SpawnActorFromClass` "/Game/Blueprints/Gun/BaseProjectile.BaseProjectile_C" (`SceneComponent.K2_GetComponentToWorld` (`self.bulletLoc`)) "Undefined" "OverrideRootScale" null null))

(event `Rotate`
  (params (axisInput :type "Float (double-precision)"))
  (bind _turretmesh (`self.turretMesh`))
  (bind _turretmesh_2 (`self.turretMesh`))
  (bind _rotangle (`self.rotAngle`))
  (bind (_returnvalue_roll _returnvalue_pitch _returnvalue_yaw) (`KismetMathLibrary.BreakRotator` (`SceneComponent.K2_GetComponentRotation` _turretmesh)))
  (bind _returnvalue (`SceneComponent.K2_GetComponentToWorld` _turretmesh_2))
  ;[1 1 1] rotate
  (`SceneComponent.K2_SetWorldRotation` _turretmesh (`KismetMathLibrary.MakeRotator` _returnvalue_roll _returnvalue_pitch (+ (* axisInput _rotangle) _rotangle)) false false)
  ;[1 1 1] clamp rotation
  (`SceneComponent.K2_SetWorldTransform` _turretmesh_2 (`KismetMathLibrary.MakeTransform` (.location _returnvalue) (`KismetMathLibrary.MakeRotator` (.roll (.rotation _returnvalue)) (.pitch (.rotation _returnvalue)) (`KismetMathLibrary.ClampAngle` (.yaw (.rotation _returnvalue)) 0.0 180.0)) (.scale _returnvalue)) true false))

(event `self.ReceiveBeginPlay`)

(fn `UserConstructionScript`)