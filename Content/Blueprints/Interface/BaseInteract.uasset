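; BaseInteract is an interaction Blueprint that shows a floating widget over a BaseCharacter detected in front of it.
; Every tick it line-traces for Pawn objects along its Arrow's forward vector up to TraceRange, toggling the Widget's visibility on whether a BaseCharacter is hit.
; The last hit character is stored as CurrentActor and never cleared, so the Widget keeps following above it even while hidden.
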(event `interact widget`
  (bind _arrow (`self.Arrow`))
  (bind _returnvalue (`SceneComponent.K2_GetComponentLocation` _arrow))
  (bind _outhit (`KismetSystemLibrary.LineTraceSingleForObjects` _returnvalue (+ _returnvalue (* (`SceneComponent.GetForwardVector` _arrow) (`self.Trace range`))) (`|MakeArray` "ObjectTypeQuery3" :!type "EObjectTypeQuery Enum")))
  (bind _asbase_character (cast `/Game/Blueprints/ThirdPersonBP/BaseCharacter` (`.HitActor` (`GameplayStatics.BreakHitResult` _outhit)))
    (:`then`
      (`SceneComponent.SetVisibility` (`self.Widget`) true false)
      (set `self.CurrentActor` _asbase_character))
    (:`CastFailed`
      (`SceneComponent.SetVisibility` (`self.Widget`) false false))))

(event `self.ReceiveTick`
  (params (DeltaSeconds :type "Float (single-precision)"))
  (bind _currentactor (`self.CurrentActor`))
  (bind (_returnvalue_x _returnvalue_y _returnvalue_z) (`KismetMathLibrary.BreakVector` (`self.K2_GetActorLocation` _currentactor)))
  (`self.interact widget`)
  (if (`KismetSystemLibrary.IsValid` _currentactor)
    (`SceneComponent.K2_SetWorldLocation` (`self.Widget`) (`KismetMathLibrary.MakeVector` _returnvalue_x _returnvalue_y (+ _returnvalue_z 150.0)) false false)))

(fn `NewFunction_0`)

(fn `UserConstructionScript`)