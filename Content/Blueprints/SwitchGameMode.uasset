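; SwitchGameMode is an actor that toggles flying mode between the player character and a FlyingPawn.
; It enables input from player controller 0 on BeginPlay and listens for the StartFly action.
; Each press alternates through a FlipFlop, setting IsFlying on the first FlyingPawn found and IsOperating on the ThirdPersonCharacter to true or false together.
; It only sets these flags and performs no possession change itself.
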(event `self.ReceiveBeginPlay`
  (`self.EnableInput` (`GameplayStatics.GetPlayerController` 0)))

(event `InputAction|StartFly`
  (params (Key :type "Key Structure"))
  (bind _returnvalue (`GameplayStatics.GetPlayerCharacter` 0))
  (:`Pressed`
    (bind _outactors (`GameplayStatics.GetAllActorsOfClass` "/Game/Blueprints/FlyingBP/Blueprints/FlyingPawn.FlyingPawn_C"))
    (`/Engine/EditorBlueprintResources/StandardMacros.FlipFlop`
      (:`A`
        (bind _output (`|GetArrayItem` _outactors))
        (set `/Game/Blueprints/FlyingBP/Blueprints/FlyingPawn.IsFlying` true _output)
        (bind _asthird_person_character (cast `/Game/Blueprints/ThirdPersonBP/ThirdPersonCharacter` _returnvalue))
        (set `/Game/Blueprints/ThirdPersonBP/ThirdPersonCharacter.IsOperating` true _asthird_person_character))
      (:`B`
        (set `/Game/Blueprints/FlyingBP/Blueprints/FlyingPawn.IsFlying` false _output)
        (bind _asthird_person_character_2 (cast `/Game/Blueprints/ThirdPersonBP/ThirdPersonCharacter` _returnvalue))
        (set `/Game/Blueprints/ThirdPersonBP/ThirdPersonCharacter.IsOperating` false _asthird_person_character_2)))))

(fn `UserConstructionScript`)