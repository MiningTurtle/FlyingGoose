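; Camera Blueprint that scrolls forward along its local X axis at the flying pawn's speed.
; BeginPlay copies CurrentForwardSpeed once from the first FlyingPawn found and stores the camera's ortho width in NewVar0, which nothing here reads.
; Tick applies a swept local offset scaled by delta time, so later changes to the pawn's speed are not picked up.
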(event `self.ReceiveBeginPlay`
  ;[1 1 1] initalize flying pawn to know the movement speed
  (bind _outactors (`GameplayStatics.GetAllActorsOfClass` "/Game/Blueprints/FlyingBP/Blueprints/FlyingPawn.FlyingPawn_C"))
  (set `self.speed` (`/Game/Blueprints/FlyingBP/Blueprints/FlyingPawn.Current forward speed` (`|GetArrayItem` _outactors)))
  ;[1 1 1] Get Camera bounds
  (bind _desiredview (`CameraComponent.GetCameraView` (`self.Camera`) 0.0))
  (set `self.NewVar_0` (`.OrthoWidth` (break `MinimalViewInfo` _desiredview))))

(event `self.ReceiveTick`
  (params (DeltaSeconds :type "Float (single-precision)"))
  ;[1 1 1] movement
  (`self.K2_AddActorLocalOffset` (`KismetMathLibrary.MakeVector` (* (`self.speed`) DeltaSeconds)) true))

(fn `UserConstructionScript`)